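; BP_Audio is an audio controller that fires a snare trigger from the head movement of a tagged skeletal mesh actor.
; On BeginPlay it finds the "Ross" actor, stores its mesh, then creates and plays an audio component as the sound generator.
; Each Tick it checks the head socket's rotation against a threshold, using a resettable DoOnce to send "SnareTrig" once per crossing.
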(event `self.ReceiveBeginPlay`
  (`|ExecutionSequence`
    (:`then_0`
      (bind _outactors (`GameplayStatics.GetAllActorsWithTag` "Ross"))
      (for _array_element _outactors
        (bind _asskeletal_mesh_actor (cast `SkeletalMeshActor` _array_element)
          (:`then`
            (set `self.RossMesh` _asskeletal_mesh_actor)
            (bind _returnvalue (`AddComponent|NODE_AddAudioComponent-0`))
            (set `self.Generator` _returnvalue))
          (:`CastFailed`
            (`KismetSystemLibrary.PrintString` "fail")))))
    (:`then_1`
      (`AudioComponent.Play` (`self.Generator`) 0.0))))

(event `self.ReceiveTick`
  (params (DeltaSeconds :type "Float (single-precision)"))
  (if (< (.y (`KismetMathLibrary.BreakRotIntoAxes` (`SceneComponent.GetSocketRotation` (`SkeletalMeshActor.SkeletalMeshComponent` (`self.RossMesh`)) "head"))) -0.5)
    (`/Engine/EditorBlueprintResources/StandardMacros.DoOnce` false :!label _label
      (:`Completed`
        (`AudioParameterControllerInterface.SetTriggerParameter` (`self.Generator`) "SnareTrig")))
    (else
      (goto _label :!via `Reset`))))

(fn `UserConstructionScript`)